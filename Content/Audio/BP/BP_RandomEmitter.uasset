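; Random ambient emitter Blueprint that plays its Sound at intervals from varying positions around its Audio component.
; BeginPlay calls a Tick event that spawns and plays the sound at a random horizontal offset from the component, keeping its height.
; Each call also sets a looping timer back to that same event with a newly randomized delay, so both timing and position vary.
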(event `self.ReceiveBeginPlay`
  (`self.Tick`))

(event `Tick`
  (bind _returnvalue (`KismetMathLibrary.RandomFloatInRange` -300.0 300.0))
  (bind (_returnvalue_x _returnvalue_y _returnvalue_z) (`KismetMathLibrary.BreakVector` (`SceneComponent.K2_GetComponentLocation` (`self.Audio`))))
  (`KismetSystemLibrary.K2_SetTimerDelegate` (delegate `Tick`) (+ 3.0 (`KismetMathLibrary.RandomFloatInRange` 5.0 8.0)) true)
  (bind _returnvalue_2 (`GameplayStatics.SpawnSoundAtLocation` (`self.Sound`) (`KismetMathLibrary.MakeVector` (+ _returnvalue_x _returnvalue) (+ _returnvalue_y _returnvalue) _returnvalue_z) (struct) 1.0 1.0 0.0 null null))
  (`AudioComponent.Play` _returnvalue_2 0.0))

(fn `UserConstructionScript`)