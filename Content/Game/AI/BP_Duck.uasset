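; BP_Duck is an AI duck Blueprint that stores state about a target and a child.
; SetTarget and SetChild events each record a flag and an object reference.
; GotTarget and GotChild functions return those stored pairs for other code to query.
; The file holds no movement or decision logic, and its construction script is empty.
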(event `/Game/Game/AI/BPI_GotTarget.SetTarget`
  (params (True :type Boolean) (Object :type "Object Object Reference"))
  (set `self.Target` True)
  (set `self.TargetObject` Object))

(event `/Game/Game/AI/BPI_GotTarget.SetChild`
  (params (True :type Boolean) (Object :type "Object Object Reference"))
  (set `self.Child` True)
  (set `self.ChildObject` Object))

(fn `GotChild`
  (returns (True :type Boolean) (Object :type "Object Object Reference"))
  (return (`self.Child`) (`self.ChildObject`)))

(fn `GotTarget`
  (returns (True :type Boolean) (Object :type "Object Object Reference"))
  (return (`self.Target`) (`self.TargetObject`)))

(fn `UserConstructionScript`)