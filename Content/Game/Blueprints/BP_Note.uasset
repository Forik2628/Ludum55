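; BP_Note is a note actor that reveals its text while the player character, BP_Ludum_Character, overlaps it.
; Its TextRender and Plane components start hidden on BeginPlay.
; Overlap begin shows both and overlap end hides them, but only when the ForestNote, WaterNote and FireNote flags are all true.
; The blueprint never sets these flags itself.
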(event `self.ReceiveBeginPlay`
  (`SceneComponent.SetVisibility` (`self.TextRender`) false false)
  (`SceneComponent.SetVisibility` (`self.Plane`) false false))

(event `self.ReceiveActorBeginOverlap`
  (params (OtherActor :type "Actor Object Reference"))
  (cast `/Game/Game/Character/BP_Ludum_Character` OtherActor)
  (if (`self.ForestNote`)
    (if (`self.WaterNote`)
      (if (`self.FireNote`)
        (`SceneComponent.SetVisibility` (`self.TextRender`) true false)
        (`SceneComponent.SetVisibility` (`self.Plane`) true false)))))

(event `self.ReceiveActorEndOverlap`
  (params (OtherActor :type "Actor Object Reference"))
  (cast `/Game/Game/Character/BP_Ludum_Character` OtherActor)
  (if (`self.ForestNote`)
    (if (`self.WaterNote`)
      (if (`self.FireNote`)
        (`SceneComponent.SetVisibility` (`self.TextRender`) false false)
        (`SceneComponent.SetVisibility` (`self.Plane`) false false)))))

(fn `UserConstructionScript`)