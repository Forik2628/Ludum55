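; BP_Idol is a pickup-style actor that unlocks a Water, Fire or Forest skill for BP_Ludum_Character.
; BeginPlay picks the idol mesh from the IdolWater, IdolFire and IdolForest booleans, separately from the IdolType enum that selects the skill.
; When the character overlaps it, a DoOnce-guarded branch sets that element's availability flag on the character and calls its matching collect event.
; The idol stays in the level afterwards.
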(event `self.ReceiveBeginPlay`
  (if (`self.Idol_Water`)
    (`StaticMeshComponent.SetStaticMesh` (`self.Cylinder`) "/Game/Game/Environment/Meshes/SM_idol_1.SM_Idol_1")
    (elif (`self.IdolFire`)
      (`StaticMeshComponent.SetStaticMesh` (`self.Cylinder`) "/Game/Game/Environment/Meshes/SM_idol_2.SM_idol_2")
      (elif (`self.IdolForest`)
        (`StaticMeshComponent.SetStaticMesh` (`self.Cylinder`) "/Game/Game/Environment/Meshes/SM_idol_3.SM_idol_3")))))

(event `self.ReceiveActorBeginOverlap`
  (params (OtherActor :type "Actor Object Reference"))
  (cast `/Game/Game/Character/BP_Ludum_Character` OtherActor)
  (switch `string` (`self.IdolType`)
    (:`FOREST`
      (`/Engine/EditorBlueprintResources/StandardMacros.DoOnce` false
        (:`Completed`
          (`self.ForestSkillActivate`))))
    (:`FIRE`
      (`/Engine/EditorBlueprintResources/StandardMacros.DoOnce` false
        (:`Completed`
          (`self.FireSkillActivate`))))
    (:`WATER`
      (`/Engine/EditorBlueprintResources/StandardMacros.DoOnce` false
        (:`Completed`
          (`self.WaterSkillActivate`))))))

(event `ForestSkillActivate`
  (`KismetSystemLibrary.PrintText` "Forest")
  (bind _returnvalue (`GameplayStatics.GetActorOfClass` "/Game/Game/Character/BP_Ludum_Character.BP_Ludum_Character_C"))
  (set `/Game/Game/Character/BP_Ludum_Character.ForestAvailable` true _returnvalue)
  (`/Game/Game/Character/BP_Ludum_Character.CollectForestEvent` _returnvalue))

(event `WaterSkillActivate`
  (`KismetSystemLibrary.PrintText` "Water")
  (bind _returnvalue (`GameplayStatics.GetActorOfClass` "/Game/Game/Character/BP_Ludum_Character.BP_Ludum_Character_C"))
  (set `/Game/Game/Character/BP_Ludum_Character.WaterAvailable` true _returnvalue)
  (`/Game/Game/Character/BP_Ludum_Character.CollectWaterEvent` _returnvalue))

(event `FireSkillActivate`
  (`KismetSystemLibrary.PrintText` "Fire")
  (bind _returnvalue (`GameplayStatics.GetActorOfClass` "/Game/Game/Character/BP_Ludum_Character.BP_Ludum_Character_C"))
  (set `/Game/Game/Character/BP_Ludum_Character.FireAvailable` true _returnvalue)
  (`/Game/Game/Character/BP_Ludum_Character.CollectFireEvent` _returnvalue))

(fn `UserConstructionScript`)