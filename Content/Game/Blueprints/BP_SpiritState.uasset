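; BP_SpiritState renders the player's fire, forest and water spirit status through a SceneCapture2D showing only its own components, and adds a WBP_Spirits widget to the viewport.
; Each tick it recaptures, refreshes the widget buttons and toggles spirit and ghost visibility from the character's availability and cooldown flags.
; The selected SkillNumber picks which spirit grows, with a timeline lerping the scales toward their target sizes.
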(event `self.ReceiveBeginPlay`
  (`SceneCaptureComponent.ShowOnlyActorComponents` (`self.SceneCaptureComponent2D`) (`ActorComponent.GetOwner` (`self.Scene`)) false)
  (bind _returnvalue (`|CreateWidget` "/Game/Game/UI/WBP_Spirits.WBP_Spirits_C"))
  (`UserWidget.AddToViewport` _returnvalue 0))

(event `self.ReceiveTick`
  (params (DeltaSeconds :type "Float (single-precision)"))
  (`SceneCaptureComponent2D.CaptureScene` (`self.SceneCaptureComponent2D`))
  (bind _asbp_ludum_character (cast `/Game/Game/Character/BP_Ludum_Character` (`GameplayStatics.GetPlayerCharacter` 0)))
  (`/Game/Game/UI/WBP_Spirits.ShowButton3` (stale `self.ReceiveBeginPlay` _returnvalue))
  (`/Game/Game/UI/WBP_Spirits.ShowButton1` (stale `self.ReceiveBeginPlay` _returnvalue))
  (`/Game/Game/UI/WBP_Spirits.ShowButton2` (stale `self.ReceiveBeginPlay` _returnvalue))
  (`SceneComponent.SetVisibility` (`self.Fire`) (`/Game/Game/Character/BP_Ludum_Character.FireAvailable` _asbp_ludum_character) false)
  (`SceneComponent.SetVisibility` (`self.Forest`) (`/Game/Game/Character/BP_Ludum_Character.ForestAvailable` _asbp_ludum_character) false)
  (`SceneComponent.SetVisibility` (`self.Water`) (`/Game/Game/Character/BP_Ludum_Character.WaterAvailable` _asbp_ludum_character) false)
  (`SceneComponent.SetVisibility` (`self.ForestGhost`) (not (`/Game/Game/Character/BP_Ludum_Character.ForestCD` _asbp_ludum_character)) false)
  (`SceneComponent.SetVisibility` (`self.WaterGhost`) (not (`/Game/Game/Character/BP_Ludum_Character.WaterCD` _asbp_ludum_character)) false)
  (`SceneComponent.SetVisibility` (`self.FireGhost`) (not (`/Game/Game/Character/BP_Ludum_Character.FireCD` _asbp_ludum_character)) false)
  (switch `int` (`/Game/Game/Character/BP_Ludum_Character.SkillNumber` _asbp_ludum_character)
    (:`0`
      (`self.SetAllLittle`))
    (:`1`
      (`self.SetBigForest`))
    (:`2`
      (`self.SetBigWater`))
    (:`3`
      (`self.SetBigFire`)))
  (`self.SetSizes`))

(event `SetSizes`
  (bind _fire (`self.Fire`))
  (bind _water (`self.Water`))
  (bind _forest (`self.Forest`))
  (bind (_returnvalue_location _returnvalue_rotation _returnvalue_scale) (`KismetMathLibrary.BreakTransform` (`SceneComponent.GetRelativeTransform` _fire)))
  (bind (_returnvalue_location_2 _returnvalue_rotation_2 _returnvalue_scale_2) (`KismetMathLibrary.BreakTransform` (`SceneComponent.GetRelativeTransform` _forest)))
  (bind (_returnvalue_location_3 _returnvalue_rotation_3 _returnvalue_scale_3) (`KismetMathLibrary.BreakTransform` (`SceneComponent.GetRelativeTransform` _water)))
  (bind (_direction _newtrack_0) (`Timeline|Timeline` :!via `PlayFromStart`)
    (:`Update`
      (`SceneComponent.SetRelativeScale3D` _fire (`KismetMathLibrary.VLerp` _returnvalue_scale (`self.FireSize`) _newtrack_0))
      (`SceneComponent.SetRelativeScale3D` _water (`KismetMathLibrary.VLerp` _returnvalue_scale_3 (`self.WaterSize`) _newtrack_0))
      (`SceneComponent.SetRelativeScale3D` _forest (`KismetMathLibrary.VLerp` _returnvalue_scale_2 (`self.ForestSize`) _newtrack_0)))))

(event `SetBigWater`
  (bind _standartsize (`self.StandartSize`))
  (set `self.FireSize` _standartsize)
  (set `self.WaterSize` (`self.BigSize`))
  (set `self.ForestSize` _standartsize))

(event `SetBigFire`
  (bind _standartsize (`self.StandartSize`))
  (set `self.FireSize` (`self.BigSize`))
  (set `self.WaterSize` _standartsize)
  (set `self.ForestSize` _standartsize))

(event `SetBigForest`
  (bind _standartsize (`self.StandartSize`))
  (set `self.FireSize` _standartsize)
  (set `self.WaterSize` _standartsize)
  (set `self.ForestSize` (`self.BigSize`)))

(event `SetAllLittle`
  (bind _standartsize (`self.StandartSize`))
  (set `self.FireSize` _standartsize)
  (set `self.WaterSize` _standartsize)
  (set `self.ForestSize` _standartsize))

(fn `UserConstructionScript`)