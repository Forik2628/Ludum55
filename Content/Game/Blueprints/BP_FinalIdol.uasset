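; BP_FinalIdol is the final idol actor, which triggers the player character's final event when touched.
; On BeginPlay it gives the idol mesh a dynamic instance of the main idol material.
; Capsule overlap with BP_Ludum_Character calls that character's FinalEvent.
; A separate EmissionON event uses a timeline to drive the material's Emission parameter for a glow, with no active call in this graph.
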(event `self.ReceiveBeginPlay`
  (bind _returnvalue (`KismetMaterialLibrary.CreateDynamicMaterialInstance` "/Game/Game/Environment/Materials/MI_Main_Idol.MI_Main_Idol"))
  (set `self.SetMat` _returnvalue)
  (`PrimitiveComponent.SetMaterial` (`self.FinalIdol`) 0 _returnvalue))

(event `EmissionON`
  (bind (_direction _newtrack_0) (`Timeline|Timeline`)
    (:`Update`
      (`MaterialInstanceDynamic.SetScalarParameterValue` (`self.SetMat`) "Emission" (`KismetMathLibrary.Lerp` 0.0 5.0 _newtrack_0)))))

(event `self.Capsule.OnComponentBeginOverlap`
  (params (OverlappedComponent :type "PrimitiveComponent Object Reference") (OtherActor :type "Actor Object Reference") (OtherComp :type "PrimitiveComponent Object Reference") (OtherBodyIndex :type Integer) (bFromSweep :type Boolean) (SweepResult :type "HitResult Structure (by ref)"))
  (bind _asbp_ludum_character (cast `/Game/Game/Character/BP_Ludum_Character` OtherActor))
  (`/Game/Game/Character/BP_Ludum_Character.FinalEvent` _asbp_ludum_character))

(fn `UserConstructionScript`)