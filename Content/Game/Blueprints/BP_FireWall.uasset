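; BP_FireWall is a wall that burns away when the player triggers the firewall dispatcher while standing inside its Box volume.
; On BeginPlay, or when RespawnWalls is called, it binds Burn to that dispatcher on BP_Ludum_Character actors.
; Burn checks the player overlap, then once swaps the three cube meshes to an appearance material and destroys the actor after a short delay.
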(event `self.ReceiveBeginPlay`
  (bind _outactors (`GameplayStatics.GetAllActorsOfClass` "/Game/Game/Character/BP_Ludum_Character.BP_Ludum_Character_C" :!label _label))
  (add `/Game/Game/Character/BP_Ludum_Character.FirewallDispatcher` _outactors (delegate `Burn`)))

(event `RespawnWalls`
  (goto _label))

(event `Burn`
  (if (`PrimitiveComponent.IsOverlappingActor` (`self.Box`) (`GameplayStatics.GetPlayerCharacter` 0))
    (`/Engine/EditorBlueprintResources/StandardMacros.DoOnce` false
      (:`Completed`
        (`PrimitiveComponent.SetMaterial` (`self.Cube`) 0 "/Game/Game/VFX/Character_Appearance_Dissolve/Materials/Standart/M_Appearance_10_Inst.M_Appearance_10_Inst")
        (`PrimitiveComponent.SetMaterial` (`self.Cube1`) 0 "/Game/Game/VFX/Character_Appearance_Dissolve/Materials/Standart/M_Appearance_10_Inst.M_Appearance_10_Inst")
        (`PrimitiveComponent.SetMaterial` (`self.Cube2`) 0 "/Game/Game/VFX/Character_Appearance_Dissolve/Materials/Standart/M_Appearance_10_Inst.M_Appearance_10_Inst")
        (`KismetSystemLibrary.Delay` 1.0)
        (`self.K2_DestroyActor`)))))

(fn `UserConstructionScript`)