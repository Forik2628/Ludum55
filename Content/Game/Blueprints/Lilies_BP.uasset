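; Lilies actor that reacts to the emerge event dispatcher of the BP_Idol found in the level at BeginPlay.
; When Emerge fires with IsEmerged set, it clears the flag, teleports up, then drops back after a short delay and toggles the flag again.
; When the flag is unset, Emerge only toggles it and prints a debug message, leaving the actor in place.
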(event `self.ReceiveBeginPlay`
  (bind _returnvalue (`GameplayStatics.GetActorOfClass` "/Game/Game/Blueprints/BP_Idol.BP_Idol_C"))
  (add `/Game/Game/Blueprints/BP_Idol.EmergeDispatcher` _returnvalue (delegate `Emerge`)))

(event `Emerge`
  (bind _returnvalue (`self.K2_GetActorLocation`))
  (bind _returnvalue_2 (not (`self.isEmerged`)))
  (`KismetSystemLibrary.PrintText` "Lilies_UP")
  (if (`self.isEmerged`)
    (`KismetSystemLibrary.PrintText` "Lilies_UP")
    (set `self.isEmerged` _returnvalue_2)
    (`self.K2_SetActorLocation` (+ _returnvalue (0.0 0.0 100.0)) false true)
    (`KismetSystemLibrary.Delay` 1.0)
    (`self.K2_SetActorLocation` (- _returnvalue (0.0 0.0 100.0)) false true)
    (set `self.isEmerged` (not (`self.isEmerged`)))
    (else
      (`KismetSystemLibrary.PrintText` "Lilies_DOWN")
      (set `self.isEmerged` _returnvalue_2))))

(fn `UserConstructionScript`)