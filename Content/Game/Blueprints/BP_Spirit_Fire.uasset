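; Fire spirit companion that follows the Ludum character and stays hidden until ActivateGhost reveals its ghost mesh and light.
; A looping timeline moves the ghost along a spline around the player.
; The character's Choose dispatcher toggles selection when SkillNumber matches IdolNumber, and switches it off on the next call.
; Selection timelines blend ghost scale and dynamic-material emission between flying and buff states, with on/off sounds.
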(event `self.ReceiveTick`
  (params (DeltaSeconds :type "Float (single-precision)"))
  (bind _returnvalue (`GameplayStatics.GetActorOfClass` "/Game/Game/Character/BP_Ludum_Character.BP_Ludum_Character_C"))
  (`SceneComponent.K2_SetWorldLocation` (`self.DefaultSceneRoot`) (`SceneComponent.K2_GetComponentLocation` (`Character.CapsuleComponent` _returnvalue)) false false)
  (bind (_returnvalue_roll _returnvalue_pitch _returnvalue_yaw) (`KismetMathLibrary.BreakRotator` (`SceneComponent.K2_GetComponentRotation` (`Character.CapsuleComponent` _returnvalue))))
  (`SceneComponent.K2_SetWorldRotation` (`self.Ghost`) (`KismetMathLibrary.MakeRotator` _returnvalue_roll _returnvalue_pitch (+ _returnvalue_yaw 90.0)) false false))

(event `ActivateGhost`
  (`SceneComponent.SetVisibility` (`self.Ghost`) true false)
  (`SceneComponent.SetVisibility` (`self.PointLight`) true false))

(event `self.ReceiveBeginPlay`
  (`|ExecutionSequence`
    (:`then_0`
      (`TimelineComponent.SetPlayRate` (`self.Timeline`) (`self.TimeToMove`))
      (`SceneComponent.SetVisibility` (`self.Ghost`) false false)
      (`SceneComponent.SetRelativeScale3D` (`self.Ghost`) (`self.SpiritScaleFly`))
      (`SceneComponent.SetVisibility` (`self.PointLight`) false false)
      (bind _returnvalue (`KismetMaterialLibrary.CreateDynamicMaterialInstance` "/Game/Game/Environment/Materials/MI_Ghost_Fire.MI_Ghost_Fire"))
      (set `self.FireMat` _returnvalue)
      (`PrimitiveComponent.SetMaterial` (`self.Ghost`) 0 _returnvalue))
    (:`then_1`
      (bind _outactors (`GameplayStatics.GetAllActorsOfClass` "/Game/Game/Character/BP_Ludum_Character.BP_Ludum_Character_C"))
      (add `/Game/Game/Character/BP_Ludum_Character.ChooseDispatcher` _outactors (delegate `Choose`))
      (`self.MoveArround`))))

(event `Choose`
  (bind _returnvalue (`GameplayStatics.GetActorOfClass` "/Game/Game/Character/BP_Ludum_Character.BP_Ludum_Character_C"))
  (if (`self.Choosen`)
    (`self.Deactivate`)
    (`GameplayStatics.PlaySound2D` "/Game/Audio/Metasounds/MS_Spirit_OFF.MS_Spirit_OFF" 1.0 1.0 0.0 null null)
    (else
      (bind _output_get (set `self.Choosen` (== (`/Game/Game/Character/BP_Ludum_Character.SkillNumber` _returnvalue) (`self.IdolNumber`))))
      (if _output_get
        (`self.Activate`)
        (`GameplayStatics.PlaySound2D` "/Game/Audio/Metasounds/MS_Spirit_ON.MS_Spirit_ON" 1.0 1.0 0.0 null null)
        (`GameplayStatics.PlaySound2D` "/Game/Audio/Metasounds/Spirit/MS_FIre_Spirit.MS_FIre_Spirit" 1.0 1.0 0.0 null null)
        (else
          (`self.MoveArroundContinue`))))))

(event `MoveArroundContinue`
  (if (`self.Choosen`)
    (`self.Activate`)
    (else
      (bind (_direction _newtrack_0) (`Timeline|Timeline` :!label _label)
        (:`Update`
          (bind _output_get (set `self.CurrentPosition` (`SplineComponent.GetLocationAtTime` (`self.Spline1`) _newtrack_0 "Local" false)))
          (`SceneComponent.K2_SetRelativeLocation` (`self.Ghost`) _output_get false false))
        (:`Finished`
          (`self.MoveArround`))))))

(event `MoveArround`
  (goto _label :!via `PlayFromStart`))

(event `MoveArroundStop`)

(event `Activate`
  (`self.MoveArroundStop`)
  (bind (_direction _newtrack_0) (`Timeline|MoveToCentreTimeline` :!via `PlayFromStart`)
    (:`Update`
      (`SceneComponent.SetRelativeScale3D` (`self.Ghost`) (`KismetMathLibrary.VLerp` (`self.SpiritScaleFly`) (`self.SpiritScaleBuff`) _newtrack_0))
      (`MaterialInstanceDynamic.SetScalarParameterValue` (`self.FireMat`) "Emission" (`KismetMathLibrary.Lerp` 30.0 200.0 _newtrack_0)))))

(event `Deactivate`
  (bind (_direction _newtrack_0) (`Timeline|FromCentreTimeline` :!via `PlayFromStart`)
    (:`Update`
      (`SceneComponent.SetRelativeScale3D` (`self.Ghost`) (`KismetMathLibrary.VLerp` (`self.SpiritScaleBuff`) (`self.SpiritScaleFly`) _newtrack_0))
      (`MaterialInstanceDynamic.SetScalarParameterValue` (`self.FireMat`) "Emission" (`KismetMathLibrary.Lerp` 200.0 30.0 _newtrack_0)))
    (:`Finished`
      (set `self.Choosen` false)
      (`self.MoveArroundContinue`))))

(fn `UserConstructionScript`)