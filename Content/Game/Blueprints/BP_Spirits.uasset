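; BP_Spirits is a spirit whose sphere circles a spline until the player's skill choice selects it.
; It binds Choose to the BP_Ludum_Character dispatcher and becomes chosen when SkillNumber matches its IdolNumber.
; A looping timeline drives the spline movement, while two lerp timelines move the sphere to the local origin and back.
; Any Choose event while chosen sends it back to its saved position, where orbiting resumes.
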(event `self.ReceiveBeginPlay`
  (`|ExecutionSequence`
    (:`then_0`
      (`TimelineComponent.SetPlayRate` (`self.Timeline`) (`self.TimeToMove`)))
    (:`then_1`
      (bind _outactors (`GameplayStatics.GetAllActorsOfClass` "/Game/Game/Character/BP_Ludum_Character.BP_Ludum_Character_C"))
      (add `/Game/Game/Character/BP_Ludum_Character.ChooseDispatcher` _outactors (delegate `Choose`))
      (`self.MoveArround`))))

(event `Choose`
  (bind _returnvalue (`GameplayStatics.GetActorOfClass` "/Game/Game/Character/BP_Ludum_Character.BP_Ludum_Character_C"))
  (if (`self.Choosen`)
    (`self.MoveFromCentre`)
    (else
      (bind _output_get (set `self.Choosen` (== (`/Game/Game/Character/BP_Ludum_Character.SkillNumber` _returnvalue) (`self.IdolNumber`))))
      (if _output_get
        (`self.MoveToCentre`)
        (else
          (`self.MoveArroundContinue`))))))

(event `MoveArroundContinue`
  (bind _spline (`self.Spline`))
  (bind (_direction _newtrack_0) (`Timeline|Timeline` :!label _label)
    (:`Update`
      (bind _output_get (set `self.CurrentPosition` (`SplineComponent.GetLocationAtTime` _spline _newtrack_0 "Local" false)))
      (bind _output_get_2 (set `self.CurrentRotation` (`SplineComponent.GetRotationAtTime` _spline _newtrack_0 "Local" false)))
      (`SceneComponent.K2_SetRelativeTransform` (`self.Sphere`) (`KismetMathLibrary.MakeTransform` _output_get _output_get_2) false false))
    (:`Finished`
      (`self.MoveArround`))))

(event `MoveArround`
  (if (`self.Choosen`)
    (`self.MoveToCentre`)
    (else
      (goto _label :!via `PlayFromStart`))))

(event `MoveArroundStop`
  (goto _label :!via `Stop`))

(event `MoveToCentre`
  (`self.MoveArroundStop`)
  (bind (_direction _newtrack_0) (`Timeline|MoveToCentreTimeline` :!via `PlayFromStart`)
    (:`Update`
      (`SceneComponent.K2_SetRelativeTransform` (`self.Sphere`) (`KismetMathLibrary.MakeTransform` (`KismetMathLibrary.VLerp` (`self.CurrentPosition`) (0.0 0.0 0.0) _newtrack_0) (`self.CurrentRotation`)) false false))))

(event `MoveFromCentre`
  (bind (_direction _newtrack_0) (`Timeline|FromCentreTimeline` :!via `PlayFromStart`)
    (:`Update`
      (`SceneComponent.K2_SetRelativeTransform` (`self.Sphere`) (`KismetMathLibrary.MakeTransform` (`KismetMathLibrary.VLerp` (0.0 0.0 0.0) (`self.CurrentPosition`) _newtrack_0) (`self.CurrentRotation`)) false false))
    (:`Finished`
      (set `self.Choosen` false)
      (`self.MoveArroundContinue`))))

(fn `UserConstructionScript`)