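; BP_Lilies is a lily actor that moves from a Start point to an End point when the character's swamp ability fires.
; On BeginPlay it picks a random mesh, snaps it to Start and binds LilyActivate to the BP_Ludum_Character swamp dispatcher.
; Unless WaterCD is set, LilyActivate waits up to a second at random, then lerps the mesh along a timeline scaled by TimeMove.
; RespawnLily redoes the binding.
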(event `self.ReceiveBeginPlay`
  (`|ExecutionSequence`
    (:`then_0`
      (`StaticMeshComponent.SetStaticMesh` (`self.Cube`) (`KismetArrayLibrary.Array_Random` (`self.LilyList`)))
      (`SceneComponent.K2_SetWorldLocation` (`self.Cube`) (`SceneComponent.K2_GetComponentLocation` (`self.Start`)) false false))
    (:`then_1`
      (`TimelineComponent.SetPlayRate` (`self.LiliesUp`) (`self.TimeMove`))
      (bind _outactors (`GameplayStatics.GetAllActorsOfClass` "/Game/Game/Character/BP_Ludum_Character.BP_Ludum_Character_C" :!label _label))
      (add `/Game/Game/Character/BP_Ludum_Character.SwampDispatcher` _outactors (delegate `LilyActivate`)))))

(event `RespawnLily`
  (goto _label))

(event `LilyActivate`
  (bind _returnvalue (`GameplayStatics.GetActorOfClass` "/Game/Game/Character/BP_Ludum_Character.BP_Ludum_Character_C"))
  (if (not (`/Game/Game/Character/BP_Ludum_Character.WaterCD` _returnvalue))
    (`KismetSystemLibrary.Delay` (`KismetMathLibrary.RandomFloatInRange` 0.0 1.0))
    (bind (_direction _newtrack) (`Timeline|LiliesUp` :!via `PlayFromStart`)
      (:`Update`
        (`SceneComponent.K2_SetWorldLocation` (`self.Cube`) (`KismetMathLibrary.VLerp` (`SceneComponent.K2_GetComponentLocation` (`self.Start`)) (`SceneComponent.K2_GetComponentLocation` (`self.End`)) _newtrack) false false)))))

(fn `UserConstructionScript`)