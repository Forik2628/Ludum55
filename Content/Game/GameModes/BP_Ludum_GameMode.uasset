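; BP_Ludum_GameMode is the game mode that handles player respawn and tracks the Forest, Water and Fire powers.
; It binds OnDeath to the player character's destruction, then spawns and possesses a replacement at SpawnTransform, rebinding for the next death.
; The new character is then told to respawn idols and spawn its spirit Blueprint.
; Separate events switch on a flag for each power.
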(event `Respawn`
  (bind _asbp_ludum_character (cast `/Game/Game/Character/BP_Ludum_Character` (`GameplayStatics.GetPlayerCharacter` 0) :!label _label))
  (add `self.OnDestroyed` _asbp_ludum_character (delegate `OnDeath`)))

(event `self.ReceiveBeginPlay`
  (goto _label))

(event `OnDeath` :!signature `self.OnDestroyed`
  (params (DestroyedActor :type "Actor Object Reference"))
  (bind _returnvalue (`|SpawnActorFromClass` "/Game/Game/Character/BP_Ludum_Character.BP_Ludum_Character_C" (`self.Spawn Transform`) "Undefined" "MultiplyWithRoot" null null))
  (`Controller.Possess` (`GameplayStatics.GetPlayerController` 0) _returnvalue)
  (`self.Respawn`)
  (`/Game/Game/Character/BP_Ludum_Character.RespawnIdols` _returnvalue)
  (`/Game/Game/Character/BP_Ludum_Character.SpawnSpiritBP` _returnvalue))

(event `ForestPower`
  (set `self.ForestON` true))

(event `WaterPower`
  (set `self.WaterON` true))

(event `FirePower`
  (set `self.FireON` true))

(fn `UserConstructionScript`)